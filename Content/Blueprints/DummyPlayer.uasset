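; DummyPlayer is an actor that acts as a damageable dummy, showing its remaining health through material changes.
; Each OnTakeAttack event decrements Health, then sets the Item component's material from the HealthMaterial array, indexed by Health minus one.
; When health runs out, the actor destroys itself.
; BeginPlay, overlap and Tick are disabled stubs, so all behavior comes from that one event.
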(event EventBeginPlay
  (|CallParentFunction) ; This node is disabled and will not be called.\nDrag off pins to build functionality.
)

(event Collision|EventActorBeginOverlap
  (params (OtherActor :type Actor%20Object%20Reference))
  (|CallParentFunction OtherActor) ; This node is disabled and will not be called.\nDrag off pins to build functionality.
)

(event EventTick
  (params (DeltaSeconds :type Float%20%28single-precision%29))
  (|CallParentFunction DeltaSeconds) ; This node is disabled and will not be called.\nDrag off pins to build functionality.
)

(event EventOnTakeAttack
  (bind _result (Math|Integer|DecrementInt (Variables|Default|Gethealth))
    (:%20%20
      (if (> _result 0)
        (Rendering|Material|SetMaterial (Variables|Default|GetItem) 0 (Utilities|Array|Get(acopy) (Variables|Default|GethealthMaterial) (- (Variables|Default|Gethealth) 1)))
        (else
          (Actor|DestroyActor))))))

(fn ConstructionScript
  (|CallParentFunction))