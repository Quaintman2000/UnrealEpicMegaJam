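; MyCharacter is a playable character that moves relative to the camera, turns with yaw input and calls FireWeapon on left mouse release.
; Tick grows the capsule steadily by ScalePerSecond, lengthening the camera boom at that rate and raising its socket offset over time.
; When destroyed, it spawns a new MyCharacter at the first Spawns entry, has player 0 possess it and destroys that spawn actor.
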(event EventBeginPlay)

(event Collision|EventActorBeginOverlap
  (params (OtherActor :type Actor%20Object%20Reference)))

(event EventTick
  (params (DeltaSeconds :type Float%20%28single-precision%29))
  (bind _scalepersecond (Variables|Default|GetscalePerSecond))
  (bind _cameraboom (Variables|Default|GetCameraBoom))
  (bind _returnvalue (* DeltaSeconds _scalepersecond))
  (bind _output_get (Variables|Components|Setscale (+ (Variables|Components|Getscale) _returnvalue)))
  (Transformation|SetRelativeScale3D (Variables|Default|GetCapsuleComponent) (* "1.000000,1.000000,1.000000" _output_get))
  (Variables|/Script/Engine.SpringArmComponent|SetTargetArmLength _cameraboom (+ _returnvalue (Variables|/Script/Engine.SpringArmComponent|GetTargetArmLength (Variables|Default|GetCameraBoom))))
  (Variables|/Script/Engine.SpringArmComponent|SetSocketOffset _cameraboom (Math|Vector|MakeVector 0.0 0.0 (+ DeltaSeconds (.z (Variables|/Script/Engine.SpringArmComponent|GetSocketOffset (Variables|Default|GetCameraBoom)))))))

(event EventDestroyed
  (if (> (Utilities|Array|Length (Variables|Default|Getspawns)) 0)
    (bind _returnvalue (Game|SpawnActorfromClass "MyCharacter_C" (Math|Conversions|ToTransform(Vector) (Transformation|GetActorLocation (Utilities|Array|Get(acopy) (Variables|Default|Getspawns)))) "Undefined" 0 0))
    (Pawn|Possess (Game|GetPlayerController 0) _returnvalue)
    (Actor|DestroyActor (Utilities|Array|Get(acopy) (Variables|Default|Getspawns)))))

(event Input|AxisEvents|InputAxisMoveRight
  (params (AxisValue :type Float%20%28single-precision%29))
  (Pawn|Input|AddMovementInput (Transformation|GetActorRightVector (Game|GetPlayerCameraManager 0)) AxisValue false))

(event Input|AxisEvents|InputAxisMoveForward
  (params (AxisValue :type Float%20%28single-precision%29))
  (Pawn|Input|AddMovementInput (Transformation|GetActorForwardVector (Game|GetPlayerCameraManager 0)) AxisValue false))

(event Input|AxisEvents|InputAxisTurn
  (params (AxisValue :type Float%20%28single-precision%29))
  (Pawn|Input|AddControllerYawInput AxisValue))

(event Input|MouseEvents|LeftMouseButton
  (params (Key :type Key%20Structure :default "None"))
  (:Released
    (Class|CrabCharacter|FireWeapon)))

(fn ConstructionScript)